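; BP_barter handles the player's side of bartering with a customer, setting a price offer for the item in question.
; It adds the bartering input context, caches the customer and game mode, and starts each offer at the item's base value.
; While input is unlocked, delayed increase and decrease inputs step the offer; accepting computes markup percentage and notifies the customer.
; Counter, fail and success outcomes only print text.
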(event Custom|barterSuccess
  (Development|PrintText "Success"))

(event Custom|barterCounter
  (Development|PrintText "Counter"))

(event Custom|barterFail
  (Development|PrintText "Fail"))

(event Custom|barterStart
  (bind _as_customer (Variables|Default|GetAs%20Customer))
  (bind _barteritem (Variables|/Game/Blueprints/Bartering/Chr_Customer.Chr_Customer_C|GetbarterItem _as_customer))
  (Variables|Default|SetbarterOffer (.Value (Utilities|Map|Find (Variables|/Game/Blueprints/Bartering/GM_Bartering.GM_Bartering_C|GetitemArray (Variables|Default|GetAs%20Game%20Mode)) _barteritem))) ; This sets the starting offer to the items base price
  (Development|PrintText (Utilities|Text|ToText(Name) _barteritem))
  (Variables|Default|SetinputLock true))

(event Input|EnhancedActionEvents|EnhancedInputActionIA_Increase
  (params (ActionValue :type Boolean) (ElapsedSeconds :type Float%20%28double-precision%29) (TriggeredSeconds :type Float%20%28double-precision%29) (InputAction :type Input%20Action%20Object%20Reference :default "/Game/Input/Actions/Bartering/IA_Increase.IA_Increase"))
  (if (Variables|Default|GetinputLock)
    (Utilities|FlowControl|Delay 0.075)
    (Variables|Default|SetbarterOffer (+ (Variables|Default|GetbarterOffer) 1))
    (Development|PrintText "IA_Increase")))

(event Input|EnhancedActionEvents|EnhancedInputActionIA_Decrease
  (params (ActionValue :type Boolean) (ElapsedSeconds :type Float%20%28double-precision%29) (TriggeredSeconds :type Float%20%28double-precision%29) (InputAction :type Input%20Action%20Object%20Reference :default "/Game/Input/Actions/Bartering/IA_Decrease.IA_Decrease"))
  (if (Variables|Default|GetinputLock)
    (Utilities|FlowControl|Delay 0.075)
    (Variables|Default|SetbarterOffer (- (Variables|Default|GetbarterOffer) 1))
    (Development|PrintText "IA_Decrease")))

(event Input|EnhancedActionEvents|EnhancedInputActionIA_Accept
  (params (ActionValue :type Boolean) (ElapsedSeconds :type Float%20%28double-precision%29) (TriggeredSeconds :type Float%20%28double-precision%29) (InputAction :type Input%20Action%20Object%20Reference :default "/Game/Input/Actions/Bartering/IA_Accept.IA_Accept"))
  (bind _as_customer (Variables|Default|GetAs%20Customer))
  (bind _as_game_mode (Variables|Default|GetAs%20Game%20Mode))
  (bind _barteritem (Variables|/Game/Blueprints/Bartering/Chr_Customer.Chr_Customer_C|GetbarterItem _as_customer))
  (bind _itemarray (Variables|/Game/Blueprints/Bartering/GM_Bartering.GM_Bartering_C|GetitemArray _as_game_mode))
  (bind _value (Utilities|Map|Find _itemarray _barteritem))
  (:Completed
    (if true
      (Variables|Default|Setmarkup (Math|Float|Truncate (* (/ (Math|Conversions|ToFloat(Integer) (- (Variables|Default|GetbarterOffer) _value)) (Math|Conversions|ToFloat(Integer) _value)) 1e+02))) ; Item Markup %
      (Default|BarterOffer _as_customer)
      (Variables|Default|SetinputLock false))))

(event EventBeginPlay
  (bind _asplayer_controller (Utilities|Casting|CastToPlayerController (Game|GetPlayerController 0)))
  (Input|AddMappingContext (PlayerController|LocalPlayerSubsystems|GetEnhancedInputLocalPlayerSubsystem _asplayer_controller) "/Game/Input/IMC_Bartering.IMC_Bartering" 0 "(bIgnoreAllPressedKeysUntilRelease=True,bForceImmediately=False,bNotifyUserSettings=False)")
  (bind _returnvalue (Actor|GetActorOfClass "/Game/Blueprints/Bartering/Chr_Customer.Chr_Customer_C"))
  (bind _aschr_customer (Utilities|Casting|CastToChr_Customer _returnvalue))
  (Variables|Default|SetAs%20Customer _aschr_customer)
  (bind _asgm_bartering (Utilities|Casting|CastToGM_Bartering (Game|GetGameMode)))
  (Variables|Default|SetAs%20Game%20Mode _asgm_bartering))

(fn ConstructionScript)
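; Bartering customer that haggles over a random display item and decides whether to accept the player's offer.
; On BeginPlay it sums weighted random Knowledge, Patience, Rush and Wealth rolls into TraitInfluence, picks the item from BP_barter and starts bartering next tick.
; BarterOffer rolls against Markup plus TraitInfluence for success; otherwise a second roll gives counter or fail, with each counter lowering CounterChance.
; Debug prints show a separate random roll from the deciding one.
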(event Custom|Barter%20Offer
  (bind _returnvalue (Math|Random|RandomIntegerinRange 1 100))
  (bind _as_bp_barter (Variables|Default|GetAs%20BP%20Barter))
  (bind _traitinfluence (Variables|Default|GettraitInfluence))
  (bind _markup (Variables|/Game/Blueprints/Bartering/BP_barter.BP_barter_C|Getmarkup _as_bp_barter))
  (bind _returnvalue_2 (+ _markup _traitinfluence))
  (Development|PrintText "=========================")
  (Development|PrintText "Markup")
  (Development|PrintText (Utilities|Text|ToText(Integer) _markup))
  (Development|PrintText "Trait Influence")
  (Development|PrintText (Utilities|Text|ToText(Integer) _traitinfluence))
  (Development|PrintText "Total")
  (Development|PrintText (Utilities|Text|ToText(Integer) _returnvalue_2))
  (Development|PrintText "rand int")
  (Development|PrintText (Utilities|Text|ToText(Integer) _returnvalue))
  (Development|PrintText "If random int is more than total it should say success, if it is less or equal then it should be fail or counter")
  (if (<= _returnvalue _returnvalue_2)
    (if (>= (+ (* (Variables|Default|GettraitInfluence) -1) (Variables|Default|GetcounterChance)) (Math|Random|RandomInteger 100))
      (Variables|Default|SetcounterChance (- (Variables|Default|GetcounterChance) 20))
      (Default|BarterCounter _as_bp_barter)
      (else
        (Default|BarterFail _as_bp_barter)))
    (else
      (Default|BarterSuccess _as_bp_barter))))

(event EventBeginPlay
  (bind _returnvalue (Math|Random|RandomInteger 19))
  (bind _returnvalue_2 (Actor|GetActorOfClass "/Game/Blueprints/Bartering/BP_barter.BP_barter_C"))
  (bind _asbp_barter (Utilities|Casting|CastToBP_barter _returnvalue_2))
  (Variables|Default|SetAs%20BP%20Barter _asbp_barter)
  (bind _asgm_bartering (Utilities|Casting|CastToGM_Bartering (Game|GetGameMode)))
  (Variables|Default|SetAs%20Game%20Mode _asgm_bartering)
  (Variables|Default|SettraitInfluence 0)
  ;[1 1 1] Knowledge
  (switch int _returnvalue
    (:0
      (Variables|Default|SettraitInfluence (+ (Variables|Default|GettraitInfluence) -10) :!label _label))
    (:1
      (goto _label))
    (:2
      (Variables|Default|SettraitInfluence (+ (Variables|Default|GettraitInfluence) -5) :!label _label_2))
    (:3
      (goto _label_2))
    (:4
      (goto _label_2))
    (:5
      (goto _label_2))
    (:6
      (Variables|Default|SettraitInfluence (+ (Variables|Default|GettraitInfluence) 0) :!label _label_3))
    (:7
      (goto _label_3))
    (:8
      (goto _label_3))
    (:9
      (goto _label_3))
    (:10
      (goto _label_3))
    (:11
      (goto _label_3))
    (:12
      (goto _label_3))
    (:13
      (goto _label_3))
    (:14
      (Variables|Default|SettraitInfluence (+ (Variables|Default|GettraitInfluence) 7) :!label _label_4))
    (:15
      (goto _label_4))
    (:16
      (goto _label_4))
    (:17
      (goto _label_4))
    (:18
      (Variables|Default|SettraitInfluence (+ (Variables|Default|GettraitInfluence) 15) :!label _label_5))
    (:19
      (goto _label_5)))
  ;[1 1 1] Patience
  (switch int _returnvalue
    (:0
      (Variables|Default|SettraitInfluence (+ (Variables|Default|GettraitInfluence) -10) :!label _label_6))
    (:1
      (goto _label_6))
    (:2
      (Variables|Default|SettraitInfluence (+ (Variables|Default|GettraitInfluence) -5) :!label _label_7))
    (:3
      (goto _label_7))
    (:4
      (goto _label_7))
    (:5
      (goto _label_7))
    (:6
      (Variables|Default|SettraitInfluence (+ (Variables|Default|GettraitInfluence) 0) :!label _label_8))
    (:7
      (goto _label_8))
    (:8
      (goto _label_8))
    (:9
      (goto _label_8))
    (:10
      (goto _label_8))
    (:11
      (goto _label_8))
    (:12
      (goto _label_8))
    (:13
      (goto _label_8))
    (:14
      (Variables|Default|SettraitInfluence (+ (Variables|Default|GettraitInfluence) 7) :!label _label_9))
    (:15
      (goto _label_9))
    (:16
      (goto _label_9))
    (:17
      (goto _label_9))
    (:18
      (Variables|Default|SettraitInfluence (+ (Variables|Default|GettraitInfluence) 15) :!label _label_10))
    (:19
      (goto _label_10)))
  ;[1 1 1] Rush
  (switch int _returnvalue
    (:0
      (Variables|Default|SettraitInfluence (+ (Variables|Default|GettraitInfluence) 7) :!label _label_11))
    (:1
      (goto _label_11))
    (:2
      (goto _label_11))
    (:3
      (goto _label_11))
    (:4
      (Variables|Default|SettraitInfluence (+ (Variables|Default|GettraitInfluence) 0) :!label _label_12))
    (:5
      (goto _label_12))
    (:6
      (goto _label_12))
    (:7
      (goto _label_12))
    (:8
      (goto _label_12))
    (:9
      (goto _label_12))
    (:10
      (goto _label_12))
    (:11
      (goto _label_12))
    (:12
      (goto _label_12))
    (:13
      (Variables|Default|SettraitInfluence (+ (Variables|Default|GettraitInfluence) -5) :!label _label_13))
    (:14
      (goto _label_13))
    (:15
      (goto _label_13))
    (:16
      (goto _label_13))
    (:17
      (Variables|Default|SettraitInfluence (+ (Variables|Default|GettraitInfluence) -10) :!label _label_14))
    (:18
      (goto _label_14))
    (:19
      (Variables|Default|SettraitInfluence (+ (Variables|Default|GettraitInfluence) -15))))
  ;[1 1 1] Wealth
  (switch int _returnvalue
    (:0
      (Variables|Default|SettraitInfluence (+ (Variables|Default|GettraitInfluence) 7) :!label _label_15))
    (:1
      (goto _label_15))
    (:2
      (goto _label_15))
    (:3
      (goto _label_15))
    (:4
      (Variables|Default|SettraitInfluence (+ (Variables|Default|GettraitInfluence) 0) :!label _label_16))
    (:5
      (goto _label_16))
    (:6
      (goto _label_16))
    (:7
      (goto _label_16))
    (:8
      (goto _label_16))
    (:9
      (goto _label_16))
    (:10
      (goto _label_16))
    (:11
      (goto _label_16))
    (:12
      (goto _label_16))
    (:13
      (Variables|Default|SettraitInfluence (+ (Variables|Default|GettraitInfluence) -5) :!label _label_17))
    (:14
      (goto _label_17))
    (:15
      (goto _label_17))
    (:16
      (goto _label_17))
    (:17
      (Variables|Default|SettraitInfluence (+ (Variables|Default|GettraitInfluence) -10) :!label _label_18))
    (:18
      (goto _label_18))
    (:19
      (Variables|Default|SettraitInfluence (+ (Variables|Default|GettraitInfluence) -15))))
  ;[1 1 1] Choose item from display
  (Variables|Default|SetbarterItem (Utilities|Array|Get(acopy) (Variables|/Game/Blueprints/Bartering/BP_barter.BP_barter_C|GetdisplayItems (Variables|Default|GetAs%20BP%20Barter)) (Math|Random|RandomInteger (Utilities|Array|Length (Variables|/Game/Blueprints/Bartering/BP_barter.BP_barter_C|GetdisplayItems (Variables|Default|GetAs%20BP%20Barter))))))
  (Utilities|FlowControl|DelayUntilNextTick)
  (Default|BarterStart (Variables|Default|GetAs%20BP%20Barter)))

(fn ConstructionScript)
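; Customer character for a barter system that decides whether to accept, counter or reject the player's price offer.
; On BeginPlay it makes weighted d20 rolls for Knowledge, Patience, Rush and Wealth, chaining their modifiers into TraitInfluence.
; BarterOffer adds TraitInfluence to the markup over the GameMode's item value and rolls against it for refusal.
; A refusal rolls CounterChance minus TraitInfluence for a counter, which lowers CounterChance, and reports the outcome to the player.
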(event Custom|Barter%20Offer
  (bind _as_player (Variables|Default|GetAs%20Player))
  (bind _as_game_mode (Variables|Default|GetAs%20Game%20Mode))
  (bind _as_player_2 (Variables|Default|GetAs%20Player))
  (bind _barteritem (Variables|/Game/Characters/c0010/BP_c0010.BP_c0010_C|GetbarterItem _as_player_2))
  (bind _itemarray (Variables|/Game/Blueprints/GM_Default.GM_Default_C|GetitemArray _as_game_mode))
  (bind _value (Utilities|Map|Find _itemarray _barteritem))
  (if (<= (Math|Random|RandomInteger 100) (+ (/ (- (Variables|/Game/Characters/c0010/BP_c0010.BP_c0010_C|GetbarterOffer _as_player_2) _value) _value) (Variables|Default|GettraitInfluence)))
    (if (>= (+ (* (Variables|Default|GettraitInfluence) -1) (Variables|Default|GetcounterChance)) (Math|Random|RandomInteger 100))
      (Variables|Default|SetcounterChance (- (Variables|Default|GetcounterChance) 20))
      (Default|BarterCounter _as_player)
      (else
        (Default|BarterFail _as_player)))
    (else
      (Default|BarterSuccess _as_player))))

(event EventBeginPlay
  (bind _returnvalue (Math|Random|RandomInteger 20))
  (bind _asbp_c_0010 (Utilities|Casting|CastToBP_c0010 (Game|GetPlayerCharacter 0)))
  (Variables|Default|SetAs%20Player _asbp_c_0010)
  (bind _asgm_default (Utilities|Casting|CastToGM_Default (Game|GetGameMode)))
  (Variables|Default|SetAs%20Game%20Mode _asgm_default)
  (Variables|Default|SettraitInfluence 0)
  ;[1 1 1] Knowledge
  (switch int _returnvalue
    (:1
      (bind _value (Utilities|ExecuteAdd 0 -10 :!label _label)
        (:Out
          _)))
    (:2
      (goto _label))
    (:3
      (bind _value_2 (Utilities|ExecuteAdd 0 -5 :!label _label_2)
        (:Out
          _)))
    (:4
      (goto _label_2))
    (:5
      (goto _label_2))
    (:6
      (goto _label_2))
    (:7
      (bind _value_3 (Utilities|ExecuteAdd :!label _label_3)
        (:Out
          _)))
    (:8
      (goto _label_3))
    (:9
      (goto _label_3))
    (:10
      (goto _label_3))
    (:11
      (goto _label_3))
    (:12
      (goto _label_3))
    (:13
      (goto _label_3))
    (:14
      (goto _label_3))
    (:15
      (bind _value_4 (Utilities|ExecuteAdd 0 7 :!label _label_4)
        (:Out
          _)))
    (:16
      (goto _label_4))
    (:17
      (goto _label_4))
    (:18
      (goto _label_4))
    (:19
      (bind _value_5 (Utilities|ExecuteAdd 0 15 :!label _label_5)
        (:Out
          _)))
    (:20
      (goto _label_5)))
  ;[1 1 1] Patience
  (switch int _returnvalue
    (:1
      (bind _value_6 (Utilities|ExecuteAdd (+ _value _value_2 _value_3 _value_4 _value_5) -10 :!label _label_6)
        (:Out
          _)))
    (:2
      (goto _label_6))
    (:3
      (bind _value_7 (Utilities|ExecuteAdd (+ _value _value_2 _value_3 _value_4 _value_5) -5 :!label _label_7)
        (:Out
          _)))
    (:4
      (goto _label_7))
    (:5
      (goto _label_7))
    (:6
      (goto _label_7))
    (:7
      (bind _value_8 (Utilities|ExecuteAdd (+ _value _value_2 _value_3 _value_4 _value_5) :!label _label_8)
        (:Out
          _)))
    (:8
      (goto _label_8))
    (:9
      (goto _label_8))
    (:10
      (goto _label_8))
    (:11
      (goto _label_8))
    (:12
      (goto _label_8))
    (:13
      (goto _label_8))
    (:14
      (goto _label_8))
    (:15
      (bind _value_9 (Utilities|ExecuteAdd (+ _value _value_2 _value_3 _value_4 _value_5) 7 :!label _label_9)
        (:Out
          _)))
    (:16
      (goto _label_9))
    (:17
      (goto _label_9))
    (:18
      (goto _label_9))
    (:19
      (bind _value_10 (Utilities|ExecuteAdd (+ _value _value_2 _value_3 _value_4 _value_5) 15 :!label _label_10)
        (:Out
          _)))
    (:20
      (goto _label_10)))
  ;[1 1 1] Rush
  (switch int _returnvalue
    (:1
      (bind _value_11 (Utilities|ExecuteAdd (+ _value_6 _value_7 _value_8 _value_9 _value_10) 7 :!label _label_11)
        (:Out
          _)))
    (:2
      (goto _label_11))
    (:3
      (goto _label_11))
    (:4
      (goto _label_11))
    (:5
      (bind _value_12 (Utilities|ExecuteAdd (+ _value_6 _value_7 _value_8 _value_9 _value_10) :!label _label_12)
        (:Out
          _)))
    (:6
      (goto _label_12))
    (:7
      (goto _label_12))
    (:8
      (goto _label_12))
    (:9
      (goto _label_12))
    (:10
      (goto _label_12))
    (:11
      (goto _label_12))
    (:12
      (goto _label_12))
    (:13
      (goto _label_12))
    (:14
      (bind _value_13 (Utilities|ExecuteAdd (+ _value_6 _value_7 _value_8 _value_9 _value_10) -5 :!label _label_13)
        (:Out
          _)))
    (:15
      (goto _label_13))
    (:16
      (goto _label_13))
    (:17
      (goto _label_13))
    (:18
      (bind _value_14 (Utilities|ExecuteAdd (+ _value_6 _value_7 _value_8 _value_9 _value_10) -10 :!label _label_14)
        (:Out
          _)))
    (:19
      (goto _label_14))
    (:20
      (bind _value_15 (Utilities|ExecuteAdd (+ _value_6 _value_7 _value_8 _value_9 _value_10) -15)
        (:Out
          _))))
  ;[1 1 1] Wealth
  (switch int _returnvalue
    (:1
      (bind _value_16 (Utilities|ExecuteAdd (+ _value_11 _value_12 _value_13 _value_14 _value_15) 7 :!label _label_15)
        (:Out
          _)))
    (:2
      (goto _label_15))
    (:3
      (goto _label_15))
    (:4
      (goto _label_15))
    (:5
      (bind _value_17 (Utilities|ExecuteAdd (+ _value_11 _value_12 _value_13 _value_14 _value_15) :!label _label_16)
        (:Out
          _)))
    (:6
      (goto _label_16))
    (:7
      (goto _label_16))
    (:8
      (goto _label_16))
    (:9
      (goto _label_16))
    (:10
      (goto _label_16))
    (:11
      (goto _label_16))
    (:12
      (goto _label_16))
    (:13
      (goto _label_16))
    (:14
      (bind _value_18 (Utilities|ExecuteAdd (+ _value_11 _value_12 _value_13 _value_14 _value_15) -5 :!label _label_17)
        (:Out
          _)))
    (:15
      (goto _label_17))
    (:16
      (goto _label_17))
    (:17
      (goto _label_17))
    (:18
      (bind _value_19 (Utilities|ExecuteAdd (+ _value_11 _value_12 _value_13 _value_14 _value_15) -10 :!label _label_18)
        (:Out
          _)))
    (:19
      (goto _label_18))
    (:20
      (bind _value_20 (Utilities|ExecuteAdd (+ _value_11 _value_12 _value_13 _value_14 _value_15) -15)
        (:Out
          _))))
  (Variables|Default|SettraitInfluence (+ _value_16 _value_17 _value_18 _value_19 _value_20)))

(fn ConstructionScript)
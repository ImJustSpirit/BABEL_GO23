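; BP_Database stores dialogue state and drives a placeholder test dialogue that leads into bartering.
; Init caches the player pawn as BP_barter, and Dia_BarterStart adds a W_Bartering widget, fills the name, body and response slots with their effects, then calls BarterStart on the pawn when the dialogue outputs.
; Destroy Widget only pulses a DestoryDialogue flag true then false, and debug prints mark each stage.
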(event EventInit
  (Utilities|FlowControl|Sequence
    (:then_0
      (|CasttoBarter))))

(event Custom|Dia_BarterStart
  (Development|PrintText "Hello")
  (Utilities|CreateWidget)
  (Development|PrintText "Hello")
  (Utilities|Dialogue "Test" "This is a test, wow!" "/Game/TempFilesDELETE/temp_redChar.temp_redChar" 0 "/Game/TempFilesDELETE/temp_blankChar.temp_blankChar" 0 "/Game/TempFilesDELETE/temp_blankChar.temp_blankChar" 0 "/Game/TempFilesDELETE/temp_blankChar.temp_blankChar"
    (:Output
      (Development|PrintText "Hello")
      (Utilities|DestroyWidget)
      (Development|PrintText "Hello")
      (Default|BarterStart (Variables|Default|GetAs%20Barter)))))
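; Player character c0010, handling movement, item pickup and level warps through Enhanced Input.
; BeginPlay adds the input mapping and HUD, and caches the BP_Database game instance, which holds the inventory.
; Interact checks overlapping actors by tag: items add an ID sliced from their object name and are destroyed, warps open the level named in their second tag.
; Use Item and Pause only print debug text, the latter listing the inventory.
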(event Input|EnhancedActionEvents|EnhancedInputActionIA_Move
  (params (ActionValue :type Vector%202D%20Structure) (ElapsedSeconds :type Float%20%28double-precision%29) (TriggeredSeconds :type Float%20%28double-precision%29) (InputAction :type Input%20Action%20Object%20Reference :default "/Game/Input/Actions/IA_Move.IA_Move"))
  ;[0 0 0] Actions
  (Pawn|Input|AddMovementInput "0.000000,180.000000,0.000000" (.x ActionValue) false)
  (Pawn|Input|AddMovementInput "180.000000,0.000000,0.000000" (.y ActionValue) false))

(event Input|EnhancedActionEvents|EnhancedInputActionIA_Interact
  (params (ActionValue :type Boolean) (ElapsedSeconds :type Float%20%28double-precision%29) (TriggeredSeconds :type Float%20%28double-precision%29) (InputAction :type Input%20Action%20Object%20Reference :default "/Game/Input/Actions/IA_Interact.IA_Interact"))
  (bind _overlappingactors (Collision|GetOverlappingActors "/Script/Engine.Actor" :!class /Script/Engine.Actor))
  ;[0 0 0] Actions
  (:Started
    (for _index (range 0 (Utilities|Array|Length _overlappingactors))
      ;;[1 1 1] Item Interact
      (if (Actor|ActorHasTag (Utilities|Array|Get(acopy) _overlappingactors _index) "item")
        (Utilities|Array|Add (Variables|/Game/Blueprints/BP_Database.BP_Database_C|Getinventory (Variables|Default|GetAs%20Database)) (Utilities|String|StringToName (Utilities|String|Right (Utilities|String|Left (Utilities|GetObjectName (Utilities|Array|Get(acopy) _overlappingactors _index)) 8) 5)))
        (Actor|DestroyActor (Utilities|Array|Get(acopy) _overlappingactors _index))
        (Development|PrintString "Interact")
        (else
          ;;[1 1 1] Warp Interact
          (if (Actor|ActorHasTag (Utilities|Array|Get(acopy) _overlappingactors _index) "warp")
            (Game|OpenLevel(byName) (Utilities|Array|Get(acopy) (Variables|/Script/Engine.Actor|GetTags (Utilities|Array|Get(acopy) _overlappingactors _index)) 1))))))))

(event Input|EnhancedActionEvents|EnhancedInputActionIA_UseItem
  (params (ActionValue :type Boolean) (ElapsedSeconds :type Float%20%28double-precision%29) (TriggeredSeconds :type Float%20%28double-precision%29) (InputAction :type Input%20Action%20Object%20Reference :default "/Game/Input/Actions/IA_UseItem.IA_UseItem"))
  ;[0 0 0] Actions
  (Development|PrintString "Use Item"))

(event Input|EnhancedActionEvents|EnhancedInputActionIA_Pause
  (params (ActionValue :type Boolean) (ElapsedSeconds :type Float%20%28double-precision%29) (TriggeredSeconds :type Float%20%28double-precision%29) (InputAction :type Input%20Action%20Object%20Reference :default "/Game/Input/Actions/IA_Pause.IA_Pause"))
  (bind _as_database (Variables|Default|GetAs%20Database))
  (bind _inventory (Variables|/Game/Blueprints/BP_Database.BP_Database_C|Getinventory _as_database))
  ;[0 0 0] Actions
  (Development|PrintString "Pause")
  (for (_ _array_index) _inventory
    (Development|PrintText (Utilities|Text|ToText(Name) (Utilities|Array|Get(acopy) _inventory _array_index)))))

(event EventBeginPlay
  ;[0 0 0] BeginPlay
  (Utilities|FlowControl|Sequence
    (:then_0
      (|CallParentFunction))
    (:then_1
      (|InputMappingContext))
    (:then_2
      (|AddHUDtoViewport))
    (:then_3
      (|CasttoDatabase))))

(event Input|KeyboardEvents|DebugKeyPeriod
  (params (Key :type Key%20Structure :default "None") (ActionValue :type Input%20Action%20Value%20Structure))
  ;[0 0 0] Dev
  (:Pressed
    (if (AI|Components|NavMovement|IsMovingonGround (Variables|Character|GetCharacterMovement))
      (Development|PrintString "Is on ground")
      (else
        (Development|PrintString "Is NOT on ground")))))

(fn ConstructionScript
  (|CallParentFunction))